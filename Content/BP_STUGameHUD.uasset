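; BP_STUGameHUD is the HUD that creates the main menu, gameplay overlay and game-over screens.
; On BeginPlay it caches the game mode, then checks the level name: MenuLevel gets the main menu with cursor and UI-only input, other levels get the overlay with game-only input.
; It binds to the game mode's OnGameOver event to add the game-over widget and switch to UI input with a visible cursor.
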(event `self.ReceiveBeginPlay`
  (bind _returnvalue (`self.GetOwningPlayerController`))
  (bind _returnvalue_2 (`self.GetOwningPlayerController`))
  (`|ExecutionSequence`
    (:`then_0`
      (bind _asbp_stugame_mode_base (cast `/Game/BP_STUGameModeBase` (`GameplayStatics.GetGameMode`)))
      (set `self.GameMode` _asbp_stugame_mode_base))
    (:`then_1`
      (bind _returnvalue_3 (`GameplayStatics.GetCurrentLevelName` true))
      (if (`KismetStringLibrary.EqualEqual_StrStr` _returnvalue_3 "MenuLevel")
        (bind _returnvalue_4 (`|CreateWidget` "/Game/UI/WBP_MainMenu.WBP_MainMenu_C"))
        (`UserWidget.AddToViewport` _returnvalue_4 0)
        (`WidgetBlueprintLibrary.SetInputMode_UIOnlyEx` _returnvalue null)
        (set `PlayerController.bShowMouseCursor` true _returnvalue)
        (else
          (bind _returnvalue_5 (`|CreateWidget` "/Game/UI/WBP_GameOverlay.WBP_GameOverlay_C"))
          (`UserWidget.AddToViewport` _returnvalue_5 0)
          (`WidgetBlueprintLibrary.SetInputMode_GameOnly` _returnvalue_2)
          (set `PlayerController.bShowMouseCursor` false _returnvalue_2))))
    (:`then_2`
      (add `/Game/BP_STUGameModeBase.OnGameOver` (`self.GameMode`) (delegate `GameOver`)))))

(event `self.ReceiveTick`
  (params (DeltaSeconds :type "Float (single-precision)")))

(event `GameOver`
  (bind _returnvalue (`self.GetOwningPlayerController`))
  (bind _returnvalue_2 (`|CreateWidget` "/Game/UI/WBP_GameOver.WBP_GameOver_C"))
  (`UserWidget.AddToViewport` _returnvalue_2 0)
  (`WidgetBlueprintLibrary.SetInputMode_UIOnlyEx` _returnvalue null)
  (set `PlayerController.bShowMouseCursor` true _returnvalue))

(fn `UserConstructionScript`)