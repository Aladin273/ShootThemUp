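; BP_STUGameInstance is a game instance Blueprint that initializes user graphics and audio settings when the game starts.
; One second after Init, it loads BetterGameUserSettings and, on first launch only, sets default scalability and music and SFX volumes, then clears the first-launch flag.
; It then sets the master sound mix, hands it and the music and SFX sound classes to the settings object, and applies the settings.
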(event `self.ReceiveInit`
  (`KismetSystemLibrary.Delay` 1.0)
  (bind _returnvalue (`BetterGameUserSettings.GetBetterGameUserSettings`))
  (`|ExecutionSequence`
    (:`then_0`
      (`GameUserSettings.LoadSettings` _returnvalue false)
      (if (`BetterGameUserSettings.GetInitLaunch` _returnvalue)
        (`GameUserSettings.SetOverallScalabilityLevel` _returnvalue 3)
        (`BetterGameUserSettings.SetMusicVolume` _returnvalue 0.5)
        (`BetterGameUserSettings.SetSFXVolume` _returnvalue 0.5)
        (`BetterGameUserSettings.SetInitLaunch` _returnvalue false)))
    (:`then_1`
      (`GameplayStatics.SetBaseSoundMix` "/Game/Audio/SCM_Master.SCM_Master")
      (`BetterGameUserSettings.SetMasterSoundMix` _returnvalue "/Game/Audio/SCM_Master.SCM_Master")
      (`BetterGameUserSettings.SetMusicSoundClass` _returnvalue "/Game/Audio/SC_Music.SC_Music")
      (`BetterGameUserSettings.SetSFXSoundClass` _returnvalue "/Game/Audio/SC_SFX.SC_SFX")
      (`GameUserSettings.ApplySettings` _returnvalue false))))